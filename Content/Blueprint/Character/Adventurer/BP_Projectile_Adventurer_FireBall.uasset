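; Fireball projectile for the Adventurer character that damages Goblin players on contact.
; Sphere overlap is handled only on the server, which applies a base damage set at BeginPlay when the other actor is a Goblin player.
; A hit calls a multicast-named event to spawn an explosion emitter at the projectile, then hides the actor and destroys it after a short delay.
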(event OnComponentBeginOverlap(Sphere)
  (params (OverlappedComponent :type Primitive%20Component%20Object%20Reference) (OtherActor :type Actor%20Object%20Reference) (OtherComp :type Primitive%20Component%20Object%20Reference) (OtherBodyIndex :type Integer) (bFromSweep :type Boolean) (SweepResult :type Hit%20Result%20Structure%20%28by%20ref%29))
  (Networking|SwitchHasAuthority
    (:Authority
      (bind _asbp_player_goblin (Utilities|Casting|CastToBP_Player_Goblin OtherActor))
      (Utilities|IsValid _asbp_player_goblin
        (:Is%20Valid
          (Game|Damage|ApplyDamage _asbp_player_goblin (Variables|Default|GetBaseDamage) 0 0)
          (CallFunction|SpawnParticleMulticastReq)
          (Rendering|SetActorHiddenInGame true)
          (Utilities|FlowControl|Delay 0.2)
          (Actor|DestroyActor))))))

(event Custom|SpawnParticle_Multicast_Req
  (Effects|SpawnEmitteratLocation "/Game/Another/FXVarietyPack/Particles/P_ky_explosion.P_ky_explosion" (Transformation|GetActorLocation)))

(event EventBeginPlay
  (Variables|Default|SetBaseDamage 3e+01))

(event Collision|EventActorBeginOverlap
  (params (OtherActor :type Actor%20Object%20Reference)))

(event EventTick
  (params (DeltaSeconds :type Float%20%28single-precision%29)))

(fn ConstructionScript)