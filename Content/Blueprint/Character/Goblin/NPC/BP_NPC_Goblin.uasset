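; Goblin NPC that performs a networked sword attack and damages players.
; The server request event calls a multicast event, which uses the WichServer macro to play the swing montage only on other clients, unless already playing.
; OnHit runs a small sphere overlap at AttackDirection and applies fixed damage to pawns tagged AdventurerPlayer, with debug print and drawing.
; Nothing in this graph calls the attack request or OnHit.
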(event Custom|Attack_Server_Req
  (CallFunction|AttackMulticastReq))

(event Custom|OnHit
  (bind _attackdirection (Variables|Default|GetAttackDirection))
  (bind _returnvalue (Transformation|GetWorldLocation _attackdirection))
  ;[1 1 1] OnHit한 시점에 구체 생성 및 디버깅용 드로우
  (Development|PrintString "Hello")
  (bind _outactors (Collision|SphereOverlapActors _returnvalue 2e+01 (Utilities|Array|MakeArray "ObjectTypeQuery3") 0 (Utilities|Array|MakeArray self)))
  (Rendering|Debug|DrawDebugSphere _returnvalue 2e+01 12 "(R=1.000000,G=0.000000,B=0.037799,A=1.000000)" 1.0 1.0)
  ;[1 1 1] 충돌된 액터의 태그 를 체크해서 해당 태그(AdventurerPlayer)가 있으면
  (for _array_element _outactors
    (if (Actor|ActorHasTag _array_element "AdventurerPlayer")
      ;[1 1 1] 대미지(3) 전달-> 대미지 값 변경 가능
      (Variables|Default|SetBaseDamage 3.0)
      (Game|Damage|ApplyDamage _array_element (Variables|Default|GetBaseDamage) (Game|GetPlayerController 0) self))))

(event Custom|Attack_Multicast_Req
  (Utilities|WichServer
    (:OtherClient
      (if (not (Animation|Montage|MontageIsPlaying (Components|SkeletalMesh|GetAnimInstance (Variables|Character|GetMesh)) (Variables|Default|GetCurrentPlayingMontage)))
        (Animation|Montage|MontagePlay (Components|SkeletalMesh|GetAnimInstance (Variables|Character|GetMesh)) "/Game/Blueprint/Character/Goblin/NPC/NPC_Goblin_Animation/Enemy_Anim_Sword_Combat_Swing_Montage.Enemy_Anim_Sword_Combat_Swing_Montage" 1.0 "MontageLength" 0.0 true)
        (Variables|Default|SetCurrentPlayingMontage "/Game/Blueprint/Character/Goblin/NPC/NPC_Goblin_Animation/Enemy_Anim_Sword_Combat_Swing_Montage.Enemy_Anim_Sword_Combat_Swing_Montage")))))

(event EventBeginPlay)

(event Collision|EventActorBeginOverlap
  (params (OtherActor :type Actor%20Object%20Reference)))

(event EventTick
  (params (DeltaSeconds :type Float%20%28single-precision%29)))

(fn ConstructionScript)