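; BP_NPC_AI is the AI controller for goblin NPCs, starting the BT_NPC_AI_Goblin behavior tree on BeginPlay.
; On each AI Perception update, it passes updated actors to CheckPlayerActor, which handles only those tagged AdventurerPlayer.
; That function toggles the SensedActorKey blackboard value, clearing it if already valid or otherwise storing the player, without checking whether the stimulus was gained or lost.
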(event OnPerceptionUpdated(AIPerception)
  (params (UpdatedActors :type Array%20of%20Actor%20Object%20References))
  (for _array_element UpdatedActors
    (CallFunction|CheckPlayerActor _array_element)))

(event EventBeginPlay
  (AI|RunBehaviorTree "/Game/Blueprint/Character/Goblin/NPC/NPC_AI/BT_NPC_AI_Goblin.BT_NPC_AI_Goblin"))

(event EventTick
  (params (DeltaSeconds :type Float%20%28single-precision%29)))

(fn ConstructionScript)

(fn CheckPlayerActor
  (params (SensedActor :type Actor%20Object%20Reference))
  (if (Actor|ActorHasTag SensedActor "AdventurerPlayer")
    (Utilities|IsValid (AI|Components|Blackboard|GetValueasObject (AI|GetBlackboard 0) (Utilities|Name|MakeLiteralName "SensedActorKey"))
      (:Is%20Valid
        (AI|Components|Blackboard|SetValueasObject (AI|GetBlackboard 0) (Utilities|Name|MakeLiteralName "SensedActorKey") 0))
      (:Is%20Not%20Valid
        (AI|Components|Blackboard|SetValueasObject (AI|GetBlackboard 0) (Utilities|Name|MakeLiteralName "SensedActorKey") SensedActor)))))