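; BP_Hostage is a hostage that adventurer players can carry, set down and rescue.
; Its interaction box registers the hostage with an overlapping player on the server and shows a hold-interaction widget.
; Multicasts attach it to the carrier's hand socket or drop it below their attack point, while OnRep IsCarring toggles box collision after a delay to avoid stuck widgets.
; Rescue decrements the game mode's hostage count and expires the actor.
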(event OnComponentBeginOverlap(InteractionBox)
  (params (OverlappedComponent :type Primitive%20Component%20Object%20Reference) (OtherActor :type Actor%20Object%20Reference) (OtherComp :type Primitive%20Component%20Object%20Reference) (OtherBodyIndex :type Integer) (bFromSweep :type Boolean) (SweepResult :type Hit%20Result%20Structure%20%28by%20ref%29))
  (if (not (Variables|Default|GetIsCarring))
    (Networking|SwitchHasAuthority
      (:Authority
        (bind _asbp_player_adventurer (Utilities|Casting|CastToBP_Player_Adventurer OtherActor))
        (Utilities|IsValid _asbp_player_adventurer
          (:Is%20Valid
            (Variables|Default|SetDetactedPlayer _asbp_player_adventurer)
            (Variables|/Game/Blueprint/Character/Adventurer/BP_Player_Adventurer.BP_Player_Adventurer_C|SetIsOnInteractionWidget (Variables|Default|GetDetactedPlayer) true)
            (Variables|/Game/Blueprint/Character/Adventurer/BP_Player_Adventurer.BP_Player_Adventurer_C|SetMaxHoldTime (Variables|Default|GetDetactedPlayer) (Variables|Default|GetMaxHoldTime))
            (Variables|/Game/Blueprint/Character/Adventurer/BP_Player_Adventurer.BP_Player_Adventurer_C|SetDetacted%20Actor (Variables|Default|GetDetactedPlayer) self)
            (Default|OnInteractionWidgetClient (Variables|Default|GetDetactedPlayer))))))))

(event OnComponentEndOverlap(InteractionBox)
  (params (OverlappedComponent :type Primitive%20Component%20Object%20Reference) (OtherActor :type Actor%20Object%20Reference) (OtherComp :type Primitive%20Component%20Object%20Reference) (OtherBodyIndex :type Integer))
  (CallFunction|OffIneractionWidgetReq OtherActor))

(event Custom|StopCarried_Req
  (params (CarriedActor :type BP%20Player%20Adventurer%20Object%20Reference))
  ;[1 1 1] 운반이 중단 되면 인질 캐릭터를 운반자의 공격 위치약간 아래에 위치하도록 위치조정
  (Variables|Default|SetIsCarring false)
  (CallFunction|StopCarriedMulticast CarriedActor))

(event Custom|BeCarried_Req
  (params (CarryingActor :type BP%20Player%20Adventurer%20Object%20Reference))
  ;[1 1 1] 운반이 시작되면 운반자에 Attach
  (CallFunction|BeCarriedMulticast CarryingActor))

(event Custom|BeCarried_Multicast
  (params (CarryingActor :type BP%20Player%20Adventurer%20Object%20Reference))
  ;[1 1 1] 운반이 시작되면 운반자에 Attach
  (Transformation|AttachComponentToComponent self (Variables|/Script/Engine.Character|GetMesh CarryingActor) "Socket_Hand_L" "SnapToTarget" "SnapToTarget" "SnapToTarget" true))

(event Custom|StopCarried_Multicast
  (params (CarriedActor :type BP%20Player%20Adventurer%20Object%20Reference))
  ;[1 1 1] 운반이 중단 되면 인질 캐릭터를 운반자의 공격 위치약간 아래에 위치하도록 위치조정
  (Transformation|DetachFromActor self "KeepRelative" "KeepRelative" "KeepRelative")
  (Transformation|SetActorRelativeLocation self (- (Transformation|GetWorldLocation (Variables|/Game/Blueprint/Character/Adventurer/BP_Player_Adventurer.BP_Player_Adventurer_C|GetAttackCollisionLocation CarriedActor)) "0, 0,120.000000")))

(event Custom|OffIneractionWidget_Req
  (params (OtherActor :type Actor%20Object%20Reference))
  (CallFunction|OffInteractionWidgetMulticast OtherActor))

(event Custom|OffInteractionWidget_Multicast
  (params (OtherActor :type Actor%20Object%20Reference))
  (bind _asbp_player_adventurer (Utilities|Casting|CastToBP_Player_Adventurer OtherActor))
  (Utilities|IsValid _asbp_player_adventurer
    (:Is%20Valid
      (bind _output_get (Variables|Default|SetDetactedPlayer _asbp_player_adventurer))
      (if (== (Variables|/Game/Blueprint/Character/Adventurer/BP_Player_Adventurer.BP_Player_Adventurer_C|GetDetacted%20Actor (Variables|Default|GetDetactedPlayer)) self)
        (Variables|/Game/Blueprint/Character/Adventurer/BP_Player_Adventurer.BP_Player_Adventurer_C|SetDetacted%20Actor (Variables|Default|GetDetactedPlayer) 0)
        (Variables|/Game/Blueprint/Character/Adventurer/BP_Player_Adventurer.BP_Player_Adventurer_C|SetIsOnInteractionWidget (Variables|Default|GetDetactedPlayer) false)
        (Default|OffInteractionWidget _output_get)))))

(event Custom|InteractionBox_Enable
  (params (Enable :type Boolean))
  ;[1 1 1] 내려놓은직후에 바로 컬리젼을 활성화시키면 BeginOverlap에 들어 오는데 EndOverlap도 들어 오게 되어 위젯이 제대로 삭제 되지 않는 문제 때문에 해당 컬리젼 활성화를 0.1 초 늦춘다.
  (Utilities|FlowControl|Delay 0.1)
  (if Enable
    (Collision|SetCollisionEnabled (Variables|Default|GetInteractionBox) "NoCollision")
    (else
      (Collision|SetCollisionEnabled (Variables|Default|GetInteractionBox) "QueryOnly"))))

(event Custom|RescueServer_Req
  ;[1 1 1] 게임모드는 서버에서만 접근 가능
  (bind _asbp_main_game_mode (Utilities|Casting|CastToBP_MainGameMode (Game|GetGameMode)))
  (Math|Integer|DecrementInt (Variables|/Game/Blueprint/GameMode/Main/BP_MainGameMode.BP_MainGameMode_C|GetCurrentHostageCount _asbp_main_game_mode)
    (:%20%20
      ;[1 1 1] 해당 인질 캐릭터는 게임상에서 삭제 처리
      (Actor|SetLifeSpan 2.0))))

(event EventBeginPlay
  (Variables|Default|SetIsCarring false))

(fn ConstructionScript)

(fn OnRepIsCarring
  (CallFunction|InteractionBoxEnable (Variables|Default|GetIsCarring)))