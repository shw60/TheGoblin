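; Main game mode for a hostage-rescue match pitting four adventurers against one player goblin.
; PostLogin spawns and possesses pawns by join order, turning extra players into observers.
; GameInit randomly fills spawn points with hostages, item boxes and NPC goblins through recursive coin-flip passes.
; A one-second timer drives wait, play and result states, pushing countdown and counts to controllers and deciding winners by rescues, time, deaths or groggy players.
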(event Custom|MainTimer
  (bind _goblinpc (Variables|Default|GetGoblinPC))
  (bind _goblinpc_2 (Variables|Default|GetGoblinPC))
  (bind _goblinpc_3 (Variables|Default|GetGoblinPC))
  (bind _goblinpc_4 (Variables|Default|GetGoblinPC))
  (switch Utilities|FlowControl|Switch|SwitchonEMainGame_PlayState (Variables|Default|GetCurrentGameState)
    (:NewEnumerator0
      ;[1 1 1] 접속자수가 최대 플레이어 수만큼 이지 체크
      (if (>= (Utilities|Array|Length (Variables|Default|GetConnectPlayers)) (Variables|Default|GetMaxPlayerCount))
        ;[1 1 1] 게임플레이 상태로 변경
        (CallFunction|SaytoAll)
        (Variables|Default|SetCurrentGameState "NewEnumerator1")
        (else
          ;[1 1 1] 다른 플레이어 입장시 까지 대기
          (CallFunction|SaytoAll "WaitingPlayer"))))
    (:NewEnumerator1
      ;[1 1 1] 게임 플레이상태에서 플레이 타임(20분) 표시, 플레이 타임은 1초씩 감소
      (CallFunction|NoticeMainPlayTime (Utilities|String|ToString(Text) (Utilities|Text|FormatText "RemainTime : {T}" (CallFunction|FormatMinSecond (Variables|Default|GetPlayTime)))))
      (Math|Integer|DecrementInt (Variables|Default|GetPlayTime)
        (:%20%20
          ;[1 1 1] 생존자 수 표시
          (CallFunction|NoticePlayerCount (Utilities|String|Append "AliveCount : " (Utilities|String|ToString(Integer) (Utilities|Array|Length (Variables|Default|GetAdventurerPlayers)))))
          ;[1 1 1] 그로기 상태가 된 플레이어 수 표시
          (CallFunction|NoticeGroggyCount (Utilities|String|Append "GroggyCount : " (Utilities|String|ToString(Integer) (Variables|Default|GetGroggyPlayerCount))))
          ;[1 1 1] 현재 인질수
          (CallFunction|NoticeHostageCount (Utilities|String|Append "HostageCount : " (Utilities|String|ToString(Integer) (Variables|Default|GetCurrentHostageCount))))
          ;[1 1 1] 구출한 인질수
          (CallFunction|NoticeRescueCount (Utilities|String|Append "ResucueCount : " (Utilities|String|ToString(Integer) (Variables|Default|GetRescueCount))))
          ;[1 1 1] 생존한 모험자 수가 0이하이거나 플레이 타임이 0이하, 그로기 상태가된 모험자 플레이어가 최대 인원수 만큼 됐을때(4명) 또는 인질수가 0이하가 되면 현재 게임 상태를 결과 상태로 변경(게임 종료 조건)
          (if (Math|Boolean|ORBoolean (<= (Utilities|Array|Length (Variables|Default|GetAdventurerPlayers)) 0) (<= (Variables|Default|GetPlayTime) 0) (>= (Variables|Default|GetRescueCount) (- (Variables|Default|GetNumSpawn_Hostage) 1)) (>= (Variables|Default|GetGroggyPlayerCount) (Utilities|Array|Length (Variables|Default|GetAdventurePC))))
            (Variables|Default|SetCurrentGameState "NewEnumerator2")))))
    (:NewEnumerator2
      (Utilities|FlowControl|Sequence
        (:then_0
          ;[1 1 1] 플레이 시간 종료후 인질이 한명이상 남아 있으면
          (if (and (<= (Variables|Default|GetPlayTime) 0) (> (Variables|Default|GetCurrentHostageCount) 0))
            ;[1 1 1] 모험자들은 패배, 고블린은 승리 처리
            (for _array_element (Variables|Default|GetAdventurePC)
              (Utilities|IsValid _array_element
                (:Is%20Valid
                  (Default|ShowLoserResult _array_element))))
            (Utilities|IsValid _goblinpc_4
              (:Is%20Valid
                (Default|ShowWinnerResult _goblinpc_4)))
            (else
              ;[1 1 1] 시간 초과가 아닌 모험자 전멸이면
              (if (<= (Utilities|Array|Length (Variables|Default|GetAdventurerPlayers)) 0)
                ;[1 1 1] 모험자들은 패배, 고블린은 승리 처리
                (for _array_element_2 (Variables|Default|GetAdventurePC)
                  (Utilities|IsValid _array_element_2
                    (:Is%20Valid
                      (Default|ShowLoserResult _array_element_2))))
                (Utilities|IsValid _goblinpc
                  (:Is%20Valid
                    (Default|ShowWinnerResult _goblinpc)))
                (else
                  ;[1 1 1] 시간 초과가 아닌 모험자 그로기 상태면
                  (if (>= (Variables|Default|GetGroggyPlayerCount) (Utilities|Array|Length (Variables|Default|GetAdventurePC)))
                    ;[1 1 1] 모험자들은 패배, 고블린은 승리 처리
                    (for _array_element_3 (Variables|Default|GetAdventurePC)
                      (Utilities|IsValid _array_element_3
                        (:Is%20Valid
                          (Default|ShowLoserResult _array_element_3))))
                    (Utilities|IsValid _goblinpc_3
                      (:Is%20Valid
                        (Default|ShowWinnerResult _goblinpc_3)))
                    (else
                      ;[1 1 1] 구출된 인질수가 스폰된 인질수보다 하나 작은수 이상이면
                      (if (>= (Variables|Default|GetRescueCount) (- (Variables|Default|GetNumSpawn_Hostage) 1))
                        ;[1 1 1] 모험자들은 승리, 고블린은 패배 처리
                        (for _array_element_4 (Variables|Default|GetAdventurePC)
                          (Utilities|IsValid _array_element_4
                            (:Is%20Valid
                              (Default|ShowWinnerResult _array_element_4))))
                        (Utilities|IsValid _goblinpc_2
                          (:Is%20Valid
                            (Default|ShowLoserResult _goblinpc_2)))))))))))
        (:then_1
          ;[1 1 1] 타이머 정지
          (Utilities|Time|ClearandInvalidateTimerbyHandle (Variables|Default|GetMainTimerHnadle)))))))

(event Custom|GameInit
  (Variables|Default|SetGroggyPlayerCount 0)
  (Variables|Default|SetPlayTime 1200)
  (Variables|Default|SetCurrentGameState "NewEnumerator0")
  (CallFunction|GetActorStartPoints)
  (CallFunction|HandleGameState "NewEnumerator0")
  (CallFunction|RandomSpawnHostage)
  (CallFunction|RandomSpawnItemBox)
  (CallFunction|RandomSpawnNPC)
  (Variables|Default|SetCurrentHostageCount (Variables|Default|GetHostageSpawnCount))
  (bind _returnvalue (Utilities|Time|SetTimerbyEvent (delegate Custom|MainTimer) 1.0 true))
  (Variables|Default|SetMainTimerHnadle _returnvalue))

(event EventBeginPlay
  (CallFunction|GameInit))

(event EventPostLogin
  (params (NewPlayer :type Player%20Controller%20Object%20Reference))
  (bind _connectplayers (Variables|Default|GetConnectPlayers))
  (bind (_outitem _outindex) (Utilities|Array|Random _connectplayers))
  ;[1 1 1] 5명까지만 로그인 허용
  (if (<= (Utilities|Array|Length (Variables|Default|GetConnectPlayers)) (- (Variables|Default|GetMaxPlayerCount) 1))
    (bind _asbp_main_player_controller (Utilities|Casting|CastToBP_MainPlayerController NewPlayer))
    (bind _returnvalue (Utilities|Array|AddUnique (Variables|Default|GetConnectPlayers) _asbp_main_player_controller))
    ;[1 1 1] 접속된 순서가 5번째이하면
    (if (< _returnvalue 4)
      ;[1 1 1] 접속 순서대로 각 플레이어 스타트 위치에 모험가 폰 생성후 빙의 및 스폰
      (for _array_element (Variables|Default|GetAdventurerPlayerStartArray)
        (if (Utilities|Name|Equal(Name) (Variables|/Script/Engine.PlayerStart|GetPlayerStartTag _array_element) (Utilities|String|StringToName (Utilities|String|ToString(Integer) _returnvalue)))
          (bind _returnvalue_2 (Game|SpawnActorfromClass "/Game/Blueprint/Character/Adventurer/BP_Player_Adventurer.BP_Player_Adventurer_C" (Transformation|GetActorTransform _array_element) "AdjustIfPossibleButAlwaysSpawn" 0 0))
          (Variables|/Game/Blueprint/Character/Adventurer/BP_Player_Adventurer.BP_Player_Adventurer_C|SetPlayerID _returnvalue_2 _returnvalue)
          (Pawn|Possess _asbp_main_player_controller _returnvalue_2)
          (Utilities|Array|AddUnique (Variables|Default|GetAdventurerPlayers) _returnvalue_2)
          (Utilities|Array|AddUnique (Variables|Default|GetAdventurePC) _asbp_main_player_controller)))
      (else
        ;[1 1 1] 마지막 접속자는 고블린으로 폰 생성후 빙의 및 스폰
        (if (Utilities|Name|Equal(Name) (Variables|/Script/Engine.PlayerStart|GetPlayerStartTag (Variables|Default|GetPlayerStart_Goblin)) "PlayerStart_Goblin")
          (bind _returnvalue_3 (Game|SpawnActorfromClass "/Game/Blueprint/Character/Goblin/BP_Player_Goblin.BP_Player_Goblin_C" (Transformation|GetActorTransform (Variables|Default|GetPlayerStart_Goblin)) "AlwaysSpawn" 0 0))
          (Pawn|Possess _asbp_main_player_controller _returnvalue_3)
          (Variables|Default|SetPlayerGoblin _returnvalue_3)
          (Variables|Default|SetGoblinPC _asbp_main_player_controller)
          (Variables|Default|SetPlayTime 1200)
          ;;[1 1 1] 마지막 인원까지 접속 완료면 게임 상태를 GamePlaying으로 변경
          (CallFunction|HandleGameState "NewEnumerator1"))))
    (else
      ;[1 1 1] 5번째 이상 입장 플레이어시 옵저버로 세팅
      (Utilities|FlowControl|Delay 1.0)
      (bind _asbp_main_player_controller_2 (Utilities|Casting|CastToBP_MainPlayerController NewPlayer))
      (Variables|/Game/Blueprint/GameMode/Main/BP_MainPlayerController.BP_MainPlayerController_C|SetIsObserver _asbp_main_player_controller_2 true)
      (Variables|/Game/Blueprint/GameMode/Main/BP_MainPlayerController.BP_MainPlayerController_C|SetIsDeveloperMode _asbp_main_player_controller_2 true)
      (Variables|/Game/Blueprint/GameMode/Main/BP_MainPlayerController.BP_MainPlayerController_C|SetObservingIndex _asbp_main_player_controller_2 _outindex)
      (Game|Player|SetViewTargetwithBlend _asbp_main_player_controller_2 _outitem 0.0 "VTBlend_Linear" 0.0 false))))

(event EventOnLogout
  (params (ExitingController :type Controller%20Object%20Reference))
  (bind _adventurepc (Variables|Default|GetAdventurePC))
  (bind _adventurerplayers (Variables|Default|GetAdventurerPlayers))
  (bind _asbp_main_player_controller (Utilities|Casting|CastToBP_MainPlayerController ExitingController))
  (Utilities|Array|RemoveItem (Variables|Default|GetConnectPlayers) _asbp_main_player_controller)
  (if (<= (Utilities|Array|Length (Variables|Default|GetConnectPlayers)) 0)
    (Utilities|FlowControl|Sequence
      (:then_0
        (bind _outactors (Actor|GetAllActorsOfClass "/Game/Blueprint/Character/Hostage/BP_Hostage.BP_Hostage_C"))
        (for _array_element _outactors
          (Actor|SetLifeSpan _array_element 0.1)))
      (:then_1
        (bind _outactors_2 (Actor|GetAllActorsOfClass "/Game/Blueprint/Item/BP_ItemBox.BP_ItemBox_C"))
        (for _array_element_2 _outactors_2
          (Actor|SetLifeSpan _array_element_2 0.1)))
      (:then_2
        (bind _outactors_3 (Actor|GetAllActorsOfClass "/Game/Blueprint/Character/Goblin/NPC/BP_NPC_Goblin.BP_NPC_Goblin_C"))
        (for _array_element_3 _outactors_3
          (Actor|SetLifeSpan _array_element_3 0.1)))
      (:then_3
        (Variables|Default|SetHostageSpawnCount 0)
        (Variables|Default|SetItemBoxSpawnCount 0)
        (Variables|Default|SetNPCSpawnCount 0)
        (Variables|Default|SetRescueCount 0))
      (:then_4
        (Variables|Default|SetCurrentSpawnPoints_Hostage (Variables|Default|GetSpawnPoints_Hostage))
        (Variables|Default|SetCurrentSpawnPoints_ItemBox (Variables|Default|GetSpawnPointsItembox))
        (Variables|Default|SetCurrentSpawnPoints_NPC (Variables|Default|GetSpawnPoints_NPC))
        (for _array_element_4 _adventurepc
          (Utilities|Array|Clear _adventurepc)
          (for _array_element_5 _adventurerplayers
            (Utilities|Array|Clear _adventurerplayers)
            (CallFunction|GameInit)))))))

(fn ConstructionScript
  (bind _outactors (Actor|GetAllActorsOfClass "/Game/Blueprint/Item/BP_SpawnPoint_Hostage.BP_SpawnPoint_Hostage_C"))
  (bind _output_get (Variables|Default|SetSpawnPoints_Hostage _outactors))
  (Variables|Default|SetCurrentSpawnPoints_Hostage _output_get)
  (bind _outactors_2 (Actor|GetAllActorsOfClass "/Game/Blueprint/Item/BP_SpawnPoint_ItemBox.BP_SpawnPoint_ItemBox_C"))
  (bind _output_get_2 (Variables|Default|SetSpawnPointsItembox _outactors_2))
  (Variables|Default|SetCurrentSpawnPoints_ItemBox _output_get_2)
  (bind _outactors_3 (Actor|GetAllActorsOfClass "/Game/Blueprint/Item/BP_SpawnPoint_NPC.BP_SpawnPoint_NPC_C"))
  (bind _output_get_3 (Variables|Default|SetSpawnPoints_NPC _outactors_3))
  (Variables|Default|SetCurrentSpawnPoints_NPC _output_get_3))

(fn SpawnPlayers
  (for _index (range 0 (- (Variables|Default|GetMaxPlayerCount) 1))
    (Variables|Default|SetIndex _index)
    (for _array_element (Variables|Default|GetAdventurerPlayerStartArray)
      (if (Utilities|Name|Equal(Name) (Variables|/Script/Engine.PlayerStart|GetPlayerStartTag _array_element) (Utilities|String|StringToName (Utilities|String|ToString(Integer) (Variables|Default|GetIndex))))
        (Class|GameplayStatics|CreatePlayer (Variables|Default|GetIndex))
        (bind _returnvalue (Game|SpawnActorfromClass "/Game/Blueprint/Character/Adventurer/BP_Player_Adventurer.BP_Player_Adventurer_C" (Transformation|GetActorTransform _array_element) "AlwaysSpawn" 0 0))
        (Pawn|Possess (Game|GetPlayerController (Variables|Default|GetIndex)) _returnvalue)
        (Utilities|Array|AddUnique (Variables|Default|GetAdventurerPlayers) _returnvalue))))
  (if (Utilities|Name|Equal(Name) (Variables|/Script/Engine.PlayerStart|GetPlayerStartTag (Variables|Default|GetPlayerStart_Goblin)) "PlayerStart_Goblin")
    (Class|GameplayStatics|CreatePlayer (Variables|Default|GetIndex))
    (bind _returnvalue_2 (Game|SpawnActorfromClass "/Game/Blueprint/Character/Goblin/BP_Player_Goblin.BP_Player_Goblin_C" (Transformation|GetActorTransform (Variables|Default|GetPlayerStart_Goblin)) "AlwaysSpawn" 0 0))
    (Pawn|Possess (Game|GetPlayerController (Variables|Default|GetIndex)) _returnvalue_2)
    (Variables|Default|SetPlayerGoblin _returnvalue_2)))

(fn GetActorStartPoints
  (bind _outactors (Actor|GetAllActorsOfClass "/Script/Engine.PlayerStart"))
  (for _array_element _outactors
    (if (Utilities|Name|Equal(Name) (Variables|/Script/Engine.PlayerStart|GetPlayerStartTag _array_element) "PlayerStart_Goblin")
      (Variables|Default|SetPlayerStart_Goblin _array_element)
      (else
        (Utilities|Array|AddUnique (Variables|Default|GetAdventurerPlayerStartArray) _array_element)))))

(fn HandleGameState
  (params (NewGameState :type EMainGame_PlayState%20Enum :default "NewEnumerator0"))
  (switch Utilities|FlowControl|Switch|SwitchonEMainGame_PlayState NewGameState
    (:NewEnumerator0
      (bind _outactors (Actor|GetAllActorsOfClass "/Game/Blueprint/Item/BP_ItemSpawnVolume.BP_ItemSpawnVolume_C"))
      (for _array_element _outactors
        (Default|SetSpawningActive _array_element false)))
    (:NewEnumerator1
      (bind _outactors_2 (Actor|GetAllActorsOfClass "/Game/Blueprint/Item/BP_ItemSpawnVolume.BP_ItemSpawnVolume_C"))
      (for _array_element_2 _outactors_2
        (Default|SetSpawningActive _array_element_2 false)))
    (:NewEnumerator2
      (bind _outactors_3 (Actor|GetAllActorsOfClass "/Game/Blueprint/Item/BP_ItemSpawnVolume.BP_ItemSpawnVolume_C"))
      (for _array_element_3 _outactors_3
        (Default|SetSpawningActive _array_element_3 false)))))

(fn GetRandomSpawnPoint
  (params (SpawnedActors :type Array%20of%20Actor%20Object%20References) (SpawnedIndexs :type Array%20of%20Integers))
  (bind (_outitem _outindex) (Utilities|Array|Random SpawnedActors))
  ;[1 1 1] 배열중 랜덤하게 요소를 하나 가져와서
  (if (== (Utilities|Array|FindItem SpawnedIndexs _outindex) -1)
    ;[1 1 1] 아니면 스폰된 인덱스배열에 넣어주고 해당 액터를 반환한다.
    (Utilities|Array|AddUnique SpawnedIndexs _outindex)
    (Utilities|Array|RemoveItem SpawnedActors _outitem)
    (return _outitem)
    (else
      ;[1 1 1] 해당 배열요소의 인덱스가 이미 스폰된 액터의 인덱스이면 재귀한다.
      (CallFunction|GetRandomSpawnPoint SpawnedActors SpawnedIndexs))))

(fn RandomSpawnHostage
  ;[1 1 1] 스폰 배열의 요소들을 하나씩 가져와서 랜덤으로 스폰할지 않할지 결정 한다.
  (for _array_element (Variables|Default|GetCurrentSpawnPoints_Hostage)
    (if (Math|Random|RandomBool)
      (Game|SpawnActorfromClass "/Game/Blueprint/Character/Hostage/BP_Hostage.BP_Hostage_C" (Transformation|GetActorTransform _array_element) "Undefined" 0 0)
      ;[1 1 1] 스폰된 배열의 요소는 배열에서 제거 한다.
      (Utilities|Array|RemoveItem (Variables|Default|GetCurrentSpawnPoints_Hostage) _array_element)
      ;[1 1 1] 스폰될때마다 카운트를 증가시키고 스폰 시킬만큼의 최대 숫자만큼 스폰됐는지 비교 해서 같으면 함수를 종료한다.
      (Math|Integer|IncrementInt (Variables|Default|GetHostageSpawnCount)
        (:%20%20
          (if (== (Variables|Default|GetNumSpawn_Hostage) (Variables|Default|GetHostageSpawnCount))
            (return))))))
  ;[1 1 1] 루프를 다돌고 나서 카운트가 스폰 시킬만큼의 최대 숫자만큼 스폰이 안된상태면 재귀한다.
  (if (== (Variables|Default|GetNumSpawn_Hostage) (Variables|Default|GetHostageSpawnCount))
    (return)
    (else
      (CallFunction|RandomSpawnHostage))))

(fn RandomSpawnItemBox
  ;[1 1 1] 스폰 배열의 요소들을 하나씩 가져와서 랜덤하게 스폰할지 않할지 결정 한다.
  (for _array_element (Variables|Default|GetCurrentSpawnPoints_ItemBox)
    (if (Math|Random|RandomBool)
      (bind _returnvalue (Game|SpawnActorfromClass "/Game/Blueprint/Item/BP_ItemBox.BP_ItemBox_C" (Transformation|GetActorTransform _array_element) "Undefined" 0 0))
      (if (Variables|Default|GetIsSetItemBatch)
        _
        (elif (Variables|/Game/Blueprint/Item/BP_SpawnPoint_ItemBox.BP_SpawnPoint_ItemBox_C|GetIsRandom _array_element)
          (Utilities|IsValid _returnvalue
            (:Is%20Valid
              (Variables|/Game/Blueprint/Item/BP_ItemBox.BP_ItemBox_C|SetIsRandom _returnvalue (Variables|/Game/Blueprint/Item/BP_SpawnPoint_ItemBox.BP_SpawnPoint_ItemBox_C|GetIsRandom _array_element))))
          (else
            (Utilities|IsValid _returnvalue
              (:Is%20Valid
                (Variables|/Game/Blueprint/Item/BP_ItemBox.BP_ItemBox_C|SetItemID _returnvalue (Variables|/Game/Blueprint/Item/BP_SpawnPoint_ItemBox.BP_SpawnPoint_ItemBox_C|GetItemID _array_element)))
              (:Is%20Not%20Valid
                (return))))))
      ;[1 1 1] 스폰된 배열의 요소는 배열에서 제거 한다.
      (Utilities|Array|RemoveItem (Variables|Default|GetCurrentSpawnPoints_ItemBox) _array_element)
      ;[1 1 1] 스폰될때마다 카운트를 증가시키고 스폰 시킬만큼의 최대 숫자만큼 스폰됐는지 비교 해서 같으면 함수를 종료한다.
      (Math|Integer|IncrementInt (Variables|Default|GetItemBoxSpawnCount)
        (:%20%20
          (if (== (Variables|Default|GetNumSpawn_ItemBox) (Variables|Default|GetItemBoxSpawnCount))
            (return))))))
  ;[1 1 1] 루프를 다돌고 나서 카운트가 스폰 시킬만큼의 최대 숫자만큼 스폰이 안된상태면 재귀한다.
  (if (== (Variables|Default|GetNumSpawn_ItemBox) (Variables|Default|GetItemBoxSpawnCount))
    (return)
    (else
      (CallFunction|RandomSpawnItemBox))))

(fn RandomSpawnHostage1
  (bind _currentspawnpoints_hostage (Variables|Default|GetCurrentSpawnPoints_Hostage))
  (bind (_outitem _outindex) (Utilities|Array|Random _currentspawnpoints_hostage))
  ;[1 1 1] 스폰시킬 숫자만큼 루프를 돌면서
  (for _index (range 0 (- (Variables|Default|GetNumSpawn_Hostage) 1))
    (Development|PrintString (Utilities|String|ToString(Integer) _outindex) true true "(R=0.000000,G=0.660000,B=1.000000,A=1.000000)" 5.0)
    (Game|SpawnActorfromClass "/Game/Blueprint/Character/Hostage/BP_Hostage.BP_Hostage_C" (Transformation|GetActorTransform _outitem) "AdjustIfPossibleButAlwaysSpawn" 0 0)
    (Utilities|Array|RemoveItem (Variables|Default|GetCurrentSpawnPoints_Hostage) _outitem)))

(fn RandomSpawnNPC
  ;[1 1 1] 스폰 배열의 요소들을 하나씩 가져와서 랜덤으로 스폰할지 않할지 결정 한다.
  (for _array_element (Variables|Default|GetCurrentSpawnPoints_NPC)
    (if (Math|Random|RandomBool)
      (Game|SpawnActorfromClass "/Game/Blueprint/Character/Goblin/NPC/BP_NPC_Goblin.BP_NPC_Goblin_C" (Transformation|GetActorTransform _array_element) "Undefined" 0 0)
      ;[1 1 1] 스폰된 배열의 요소는 배열에서 제거 한다.
      (Utilities|Array|RemoveItem (Variables|Default|GetCurrentSpawnPoints_NPC) _array_element)
      ;[1 1 1] 스폰될때마다 카운트를 증가시키고 스폰 시킬만큼의 최대 숫자만큼 스폰됐는지 비교 해서 같으면 함수를 종료한다.
      (Math|Integer|IncrementInt (Variables|Default|GetNPCSpawnCount)
        (:%20%20
          (if (== (Variables|Default|GetNumSpawn_NPC) (Variables|Default|GetNPCSpawnCount))
            (return))))))
  ;[1 1 1] 루프를 다돌고 나서 카운트가 스폰 시킬만큼의 최대 숫자만큼 스폰이 안된상태면 재귀한다.
  (if (== (Variables|Default|GetNumSpawn_NPC) (Variables|Default|GetNPCSpawnCount))
    (return)
    (else
      (CallFunction|RandomSpawnNPC))))

(fn SaytoAll
  (params (Message :type String))
  (for _array_element (Variables|Default|GetConnectPlayers)
    (Variables|/Game/Blueprint/GameMode/Main/BP_MainPlayerController.BP_MainPlayerController_C|SetNotificationFromServer _array_element Message)))

(fn NoticeMainPlayTime
  (params (CurrnetTime :type String))
  (for _array_element (Variables|Default|GetConnectPlayers)
    (Variables|/Game/Blueprint/GameMode/Main/BP_MainPlayerController.BP_MainPlayerController_C|SetMainPlayTimeFromServer _array_element CurrnetTime)))

(fn NoticePlayerCount
  (params (AdventurePlayerCount :type String))
  (for _array_element (Variables|Default|GetConnectPlayers)
    (Variables|/Game/Blueprint/GameMode/Main/BP_MainPlayerController.BP_MainPlayerController_C|SetAdventurePlayerCountFromServer _array_element AdventurePlayerCount)))

(fn FormatMinSecond
  (params (Sec :type Integer))
  (bind _returnvalue (/ Sec 60))
  (bind _returnvalue_2 (Math|Integer|%(Integer) Sec 60))
  ;[1 1 1] 남은 시간이 1분 이상
  (if (== _returnvalue 0)
    _
    (else
      (LocalVariables|SetText (Utilities|String|Append (Utilities|String|ToString(Integer) _returnvalue) "'"))))
  ;[1 1 1] 1분 이하
  (if (not (== _returnvalue_2 0))
    (bind _output_get (LocalVariables|SetText (Utilities|String|Append (LocalVariables|GetText) (Utilities|String|ToString(Integer) _returnvalue_2) "\"")))
    (return (Utilities|Text|ToText(String) _output_get))))

(fn NoticeGroggyCount
  (params (GroggyCount :type String))
  (for _array_element (Variables|Default|GetConnectPlayers)
    (Variables|/Game/Blueprint/GameMode/Main/BP_MainPlayerController.BP_MainPlayerController_C|SetGroggyPlayerCountFromServer _array_element GroggyCount)))

(fn NoticeHostageCount
  (params (HostageCount :type String))
  (for _array_element (Variables|Default|GetConnectPlayers)
    (Variables|/Game/Blueprint/GameMode/Main/BP_MainPlayerController.BP_MainPlayerController_C|SetCurrent%20HostageCount _array_element HostageCount)))

(fn NoticeRescueCount
  (params (RescueCount :type String))
  (for _array_element (Variables|Default|GetConnectPlayers)
    (Variables|/Game/Blueprint/GameMode/Main/BP_MainPlayerController.BP_MainPlayerController_C|SetRescueHostageCount _array_element RescueCount)))