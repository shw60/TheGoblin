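; Main match player controller that manages announcement and result UI and provides development cheats.
; On BeginPlay it sets game-only input and creates the announcement widget only on the Remote authority branch.
; Win and lose events show a shared result widget with matching text and background, switching to UI-only input with a cursor.
; Debug keys, gated by observer or developer flags, cycle view targets through connected players or alter GameMode groggy, timer and hostage values.
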(event Custom|ShowWinnerResult
  (bind _returnvalue (UserInterface|CreateWidget "/Game/UI/HUD/Widget_BP_GameResult.Widget_BP_GameResult_C" self "Win"))
  (UserInterface|Viewport|AddtoViewport _returnvalue 0)
  (Widget|SetVisibility (Variables|/Game/UI/HUD/Widget_BP_GameResult.Widget_BP_GameResult_C|GetBG_Win _returnvalue) "Visible")
  (Widget|SetVisibility (Variables|/Game/UI/HUD/Widget_BP_GameResult.Widget_BP_GameResult_C|GetBG_Lose _returnvalue) "Hidden")
  (Input|SetInputModeUIOnly self _returnvalue "DoNotLock")
  (Variables|Default|SetbShowMouseCursor true))

(event Custom|ShowLoserResult
  (bind _returnvalue (UserInterface|CreateWidget "/Game/UI/HUD/Widget_BP_GameResult.Widget_BP_GameResult_C" self "Lose"))
  (UserInterface|Viewport|AddtoViewport _returnvalue 0)
  (Widget|SetVisibility (Variables|/Game/UI/HUD/Widget_BP_GameResult.Widget_BP_GameResult_C|GetBG_Win _returnvalue) "Hidden")
  (Widget|SetVisibility (Variables|/Game/UI/HUD/Widget_BP_GameResult.Widget_BP_GameResult_C|GetBG_Lose _returnvalue) "Visible")
  (Input|SetInputModeUIOnly self _returnvalue "DoNotLock")
  (Variables|Default|SetbShowMouseCursor true))

(event Custom|SetObserver
  ;[1 1 1] 개발전용
  (bind _asbp_main_game_mode (Utilities|Casting|CastToBP_MainGameMode (Game|GetGameMode)))
  (bind _result (Math|Integer|IncrementInt (Variables|Default|GetObservingIndex))
    (:%20%20
      (if (> _result (Utilities|Array|Length (Variables|/Game/Blueprint/GameMode/Main/BP_MainGameMode.BP_MainGameMode_C|GetConnectPlayers _asbp_main_game_mode)))
        (bind _output_get (Variables|Default|SetObservingIndex 0))
        (Game|Player|SetViewTargetwithBlend (Utilities|Array|Get(acopy) (Variables|/Game/Blueprint/GameMode/Main/BP_MainGameMode.BP_MainGameMode_C|GetConnectPlayers _asbp_main_game_mode) _output_get) 0.0 "VTBlend_Linear" 0.0 false)
        (else
          (Game|Player|SetViewTargetwithBlend (Utilities|Array|Get(acopy) (Variables|/Game/Blueprint/GameMode/Main/BP_MainGameMode.BP_MainGameMode_C|GetConnectPlayers _asbp_main_game_mode) _result) 0.0 "VTBlend_Linear" 0.0 false))))))

(event Custom|ForceAddGroggyCount
  ;[1 1 1] 개발전용
  (bind _asbp_main_game_mode (Utilities|Casting|CastToBP_MainGameMode (Game|GetGameMode)))
  (Math|Integer|IncrementInt (Variables|/Game/Blueprint/GameMode/Main/BP_MainGameMode.BP_MainGameMode_C|GetGroggyPlayerCount _asbp_main_game_mode)))

(event Custom|ForceTimer
  ;[1 1 1] 개발전용
  (bind _asbp_main_game_mode (Utilities|Casting|CastToBP_MainGameMode (Game|GetGameMode)))
  (Variables|/Game/Blueprint/GameMode/Main/BP_MainGameMode.BP_MainGameMode_C|SetPlayTime _asbp_main_game_mode 1))

(event Custom|ForceHostageCount
  ;[1 1 1] 개발전용
  (bind _asbp_main_game_mode (Utilities|Casting|CastToBP_MainGameMode (Game|GetGameMode)))
  (Math|Integer|DecrementInt (Variables|/Game/Blueprint/GameMode/Main/BP_MainGameMode.BP_MainGameMode_C|GetCurrentHostageCount _asbp_main_game_mode)))

(event EventBeginPlay
  (bind _self self)
  (Input|SetInputModeGameOnly self)
  (Variables|Default|SetbShowMouseCursor false)
  (Networking|SwitchHasAuthority
    (:Remote
      (bind _returnvalue (UserInterface|CreateWidget "/Game/UI/HUD/Widget_BP_AnnouneMessage.Widget_BP_AnnouneMessage_C" _self _self))
      (UserInterface|Viewport|AddtoViewport _returnvalue 0))))

(event Input|ActionEvents|InputActionNextObserving
  (params (Key :type Key%20Structure :default "None"))
  ;[1 1 1] 개발전용
  (:Pressed
    (if (Variables|Default|GetIsObserver)
      (CallFunction|SetObserver))))

(event Input|ActionEvents|InputActionDevelopmentTimeKey
  (params (Key :type Key%20Structure :default "None"))
  ;[1 1 1] 개발전용
  (:Pressed
    (if (or (Variables|Default|GetIsObserver) (Variables|Default|GetIsDeveloperMode))
      (CallFunction|ForceTimer))))

(event Input|ActionEvents|InputActionDevelopmentGroggyKey
  (params (Key :type Key%20Structure :default "None"))
  ;[1 1 1] 개발전용
  (:Pressed
    (if (or (Variables|Default|GetIsObserver) (Variables|Default|GetIsDeveloperMode))
      (CallFunction|ForceAddGroggyCount))))

(event Input|ActionEvents|InputActionDevelopmentHostageKey
  (params (Key :type Key%20Structure :default "None"))
  ;[1 1 1] 개발전용
  (:Pressed
    (if (or (Variables|Default|GetIsObserver) (Variables|Default|GetIsDeveloperMode))
      (CallFunction|ForceHostageCount))))

(fn ConstructionScript)