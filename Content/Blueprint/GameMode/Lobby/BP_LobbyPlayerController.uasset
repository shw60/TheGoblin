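; Lobby player controller that plays looping lobby audio, shows the lobby UI and starts the travel to a server.
; BeginPlay blends the view to the MainCamera-tagged camera, then, on authority only, creates the lobby widget with UI-only input and a visible cursor.
; JoinServer opens LoadingMap, passing the IP address as the NextMap option instead of connecting directly.
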(event Custom|JoinServer
  (params (IpAddress :type String))
  (Game|OpenLevel(byName) "LoadingMap" true (Utilities|String|Append "NextMap=" IpAddress)))

(event EventBeginPlay
  (Audio|PlaySound2D "/Game/Sound/BGM/Lobby_Looping_Cue.Lobby_Looping_Cue" 1.0 1.0 0.0 0 0)
  (bind _outactors (Actor|GetAllActorswithTag "MainCamera"))
  (if (> (Utilities|Array|Length _outactors) 0)
    (bind _ascamera_actor (Utilities|Casting|CastToCameraActor (Utilities|Array|Get(acopy) _outactors)))
    (Game|Player|SetViewTargetwithBlend _ascamera_actor 0.0 "VTBlend_Linear" 0.0 false)
    ;[1 1 1] 해당 맵만 단독으로 띄울땐 Remote, 서버이동시엔 Authority로 지정
    (Networking|SwitchHasAuthority
      (:Authority
        (bind _returnvalue (UserInterface|CreateWidget "/Game/UI/HUD/WidgetBP_Lobby.WidgetBP_Lobby_C" self))
        (bind _output_get (Variables|Default|SetWidgetBP_Lobby _returnvalue))
        (UserInterface|Viewport|AddtoViewport _output_get 0)
        (Input|SetInputModeUIOnly self (Variables|Default|GetWidgetBP_Lobby) "DoNotLock")
        (Variables|Default|SetbShowMouseCursor true)))))

(event EventTick
  (params (DeltaSeconds :type Float%20%28single-precision%29)))

(fn ConstructionScript)