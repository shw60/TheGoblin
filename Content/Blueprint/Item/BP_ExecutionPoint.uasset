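; BP_ExecutionPoint is a trigger-box actor that marks when an Adventurer player is standing inside an execution point.
; On the server, box overlap begin and end set and clear the Adventurer's IsInExcutionPoint flag.
; They also swap AdventurePlayerState between two enum values when it matches the expected one.
; Goblin logic for a hold-to-kill interaction widget while carrying remains in the graph but never runs.
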(event OnComponentBeginOverlap(ExecutionPointBox)
  (params (OverlappedComponent :type Primitive%20Component%20Object%20Reference) (OtherActor :type Actor%20Object%20Reference) (OtherComp :type Primitive%20Component%20Object%20Reference) (OtherBodyIndex :type Integer) (bFromSweep :type Boolean) (SweepResult :type Hit%20Result%20Structure%20%28by%20ref%29))
  (Networking|SwitchHasAuthority
    (:Authority
      (bind _asbp_player_adventurer (Utilities|Casting|CastToBP_Player_Adventurer OtherActor))
      (if (Utilities|Enum|Equal(Enum) (Variables|/Game/Blueprint/Character/Adventurer/BP_Player_Adventurer.BP_Player_Adventurer_C|GetAdventurePlayerState _asbp_player_adventurer) "NewEnumerator1")
        (Variables|/Game/Blueprint/Character/Adventurer/BP_Player_Adventurer.BP_Player_Adventurer_C|SetIsInExcutionPoint _asbp_player_adventurer true)
        (Variables|/Game/Blueprint/Character/Adventurer/BP_Player_Adventurer.BP_Player_Adventurer_C|SetAdventurePlayerState _asbp_player_adventurer "NewEnumerator4")
        (else
          (Variables|/Game/Blueprint/Character/Adventurer/BP_Player_Adventurer.BP_Player_Adventurer_C|SetIsInExcutionPoint _asbp_player_adventurer true))))))

(event OnComponentEndOverlap(ExecutionPointBox)
  (params (OverlappedComponent :type Primitive%20Component%20Object%20Reference) (OtherActor :type Actor%20Object%20Reference) (OtherComp :type Primitive%20Component%20Object%20Reference) (OtherBodyIndex :type Integer))
  (Networking|SwitchHasAuthority
    (:Authority
      (bind _asbp_player_adventurer (Utilities|Casting|CastToBP_Player_Adventurer OtherActor))
      (if (Utilities|Enum|Equal(Enum) (Variables|/Game/Blueprint/Character/Adventurer/BP_Player_Adventurer.BP_Player_Adventurer_C|GetAdventurePlayerState _asbp_player_adventurer) "NewEnumerator4")
        (Variables|/Game/Blueprint/Character/Adventurer/BP_Player_Adventurer.BP_Player_Adventurer_C|SetIsInExcutionPoint _asbp_player_adventurer false)
        (Variables|/Game/Blueprint/Character/Adventurer/BP_Player_Adventurer.BP_Player_Adventurer_C|SetAdventurePlayerState _asbp_player_adventurer "NewEnumerator1")
        (else
          (Variables|/Game/Blueprint/Character/Adventurer/BP_Player_Adventurer.BP_Player_Adventurer_C|SetIsInExcutionPoint _asbp_player_adventurer false))))))

(event EventBeginPlay)

(event Collision|EventActorBeginOverlap
  (params (OtherActor :type Actor%20Object%20Reference)))

(event EventTick
  (params (DeltaSeconds :type Float%20%28single-precision%29)))

(fn ConstructionScript)