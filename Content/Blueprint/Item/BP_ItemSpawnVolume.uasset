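; BP_ItemSpawnVolume is a server-authoritative volume that spawns BP_ItemBox pickups at random points while spawning is active.
; SetSpawningActive starts a timer with a random delay from the range set in the construction script, or clears it.
; SpawnItemBox places a box with random yaw inside the WhereToSpawn bounds, skips spawning on collision, prints the point, and re-arms the timer for continuous spawning.
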(event Custom|SetSpawningActive
  (params (bShouldSpawn :type Boolean))
  (Networking|SwitchHasAuthority
    (:Authority
      (if bShouldSpawn
        (bind _output_get (Variables|Default|SetSpawnDelay (Math|Random|RandomFloatinRange (Variables|Default|GetSpawnDelayRangeLow) (Variables|Default|GetSpawnDelayRangeHigh))))
        (Utilities|Time|SetTimerbyFunctionName 0 "SpawnItemBox" _output_get)
        (else
          (Utilities|Time|ClearTimerbyFunctionName 0 "SpawnItemBox"))))))

(fn ConstructionScript
  (Networking|SwitchHasAuthority
    (:Authority
      (Variables|Default|SetSpawnDelayRangeLow 0.0)
      (Variables|Default|SetSpawnDelayRangeHigh 1e+01))))

(fn SpawnItemBox
  (Networking|SwitchHasAuthority
    (:Authority
      (bind _spawnlocation (CallFunction|GetRandomPointinVolume))
      (Development|PrintString (Utilities|String|ToString(Vector) _spawnlocation) true true "(R=0.000000,G=0.660000,B=1.000000,A=1.000000)" 5.0)
      (Game|SpawnActorfromClass "/Game/Blueprint/Item/BP_ItemBox.BP_ItemBox_C" (Math|Transform|MakeTransform _spawnlocation (Math|Rotator|MakeRotator 0.0 0.0 (Math|Random|RandomFloatinRange 0.0 3.6e+02)) "1,1,1") "DontSpawnIfColliding" 0 0)
      (CallFunction|SetSpawningActive true))))

(fn GetRandomPointinVolume
  (bind _wheretospawn (Variables|Default|GetWhereToSpawn))
  (bind (_origin _boxextent) (Collision|GetComponentBounds _wheretospawn))
  (return (Math|Random|RandomPointinBoundingBox _origin _boxextent)))